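; BP_Item is an interactable item actor with a configurable mesh, scale and two detection radii, all applied in the construction script.
; Player overlap with the inner sphere sets CanInteract true, on end overlap as well as begin, so it is never cleared here.
; The outer sphere's overlap checks and the Interaction event are empty stubs.
; BeginPlay caches the BP_PlayerCharacter reference.
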(event OnComponentBeginOverlap(outerSphereCollision)
  (params (OverlappedComponent :type Primitive%20Component%20Object%20Reference) (OtherActor :type Actor%20Object%20Reference) (OtherComp :type Primitive%20Component%20Object%20Reference) (OtherBodyIndex :type Integer) (bFromSweep :type Boolean) (SweepResult :type Hit%20Result%20Structure%20%28by%20ref%29))
  (if (== OtherActor (Game|GetPlayerCharacter 0))
    _))

(event OnComponentEndOverlap(outerSphereCollision)
  (params (OverlappedComponent :type Primitive%20Component%20Object%20Reference) (OtherActor :type Actor%20Object%20Reference) (OtherComp :type Primitive%20Component%20Object%20Reference) (OtherBodyIndex :type Integer))
  (if (== (Game|GetPlayerCharacter 0) OtherActor)
    _))

(event OnComponentBeginOverlap(innerSphereCollision)
  (params (OverlappedComponent :type Primitive%20Component%20Object%20Reference) (OtherActor :type Actor%20Object%20Reference) (OtherComp :type Primitive%20Component%20Object%20Reference) (OtherBodyIndex :type Integer) (bFromSweep :type Boolean) (SweepResult :type Hit%20Result%20Structure%20%28by%20ref%29))
  (if (== OtherActor (Game|GetPlayerCharacter 0))
    (Variables|Default|SetcanInteract true)))

(event OnComponentEndOverlap(innerSphereCollision)
  (params (OverlappedComponent :type Primitive%20Component%20Object%20Reference) (OtherActor :type Actor%20Object%20Reference) (OtherComp :type Primitive%20Component%20Object%20Reference) (OtherBodyIndex :type Integer))
  (if (== (Game|GetPlayerCharacter 0) OtherActor)
    (Variables|Default|SetcanInteract true)))

(event EventBeginPlay
  (bind _asbp_player_character (Utilities|Casting|CastToBP_PlayerCharacter (Game|GetPlayerCharacter 0)))
  (Variables|Public|Ref|SetplayerRef _asbp_player_character))

(event EventInteraction)

(fn ConstructionScript
  (bind _staticmesh (Variables|Public|Mesh|GetStaticMesh))
  (Utilities|FlowControl|Sequence
    (:then_0
      (Components|Sphere|SetSphereRadius (Variables|Default|GetinnerSphereCollision) (Variables|Public|Interaction|Settings|GetinnerSphereRadius) true)
      (Components|Sphere|SetSphereRadius (Variables|Default|GetouterSphereCollision) (Variables|Public|Interaction|Settings|GetouterSphereRadius) true))
    (:then_1
      (Components|StaticMesh|SetStaticMesh (Variables|Public|Mesh|GetStaticMesh) (Variables|Public|Mesh|GetitemMesh))
      (Transformation|SetWorldTransform _staticmesh (Math|Transform|MakeTransform (Transformation|GetWorldLocation _staticmesh) (Transformation|GetWorldRotation _staticmesh) (Variables|Public|Mesh|GetitemScale)) false false))))